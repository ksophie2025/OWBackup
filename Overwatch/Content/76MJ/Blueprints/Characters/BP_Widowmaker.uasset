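; BP_Widowmaker is a character Blueprint whose only logic is switching between first-person and third-person cameras.
; The IA_SwitchCam input drives a FlipFlop that activates one camera and deactivates the other.
; Third-person turns off controller-yaw rotation and boom pitch inheritance, while first-person turns controller-yaw rotation back on without restoring pitch inheritance.
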(event `EnhancedInput|/Game/76MJ/Input/Actions/IA_SwitchCam`
  (params (ActionValue :type Boolean) (ElapsedSeconds :type "Float (double-precision)") (TriggeredSeconds :type "Float (double-precision)") (InputAction :type "InputAction Object Reference" :default "/Game/76MJ/Input/Actions/IA_SwitchCam.IA_SwitchCam"))
  (:`Started`
    (`/Engine/EditorBlueprintResources/StandardMacros.FlipFlop`
      (:`A`
        (`ActorComponent.SetActive` (`self.ThirdPersonCamera`) true false)
        (`ActorComponent.SetActive` (`self.FirstPersonCamera`) false false)
        (set `self.bUseControllerRotationYaw` false)
        (set `SpringArmComponent.bInheritPitch` false (`self.CameraBoom`)))
      (:`B`
        (`ActorComponent.SetActive` (`self.FirstPersonCamera`) true false)
        (`ActorComponent.SetActive` (`self.ThirdPersonCamera`) false false)
        (set `self.bUseControllerRotationYaw` true)))))

(fn `UserConstructionScript`)