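; Healing pickup actor that triggers when a Player-tagged actor overlaps it, then goes on cooldown.
; Activation plays sound and effect, hides the cross, and sphere-traces for unique Player-tagged pawns, currently only printing their names without restoring health.
; A delay-based timer flag blocks retriggering until the cooldown ends and the cross reappears.
; Tick spins and bobs the cross using sine-driven offsets.
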(event `self.ReceiveBeginPlay`
  (`|ExecutionSequence`
    (:`then_0`
      (`SceneComponent.K2_AddWorldOffset` (`self.Cross`) (`KismetMathLibrary.MakeVector` 0.0 0.0 (* (`KismetMathLibrary.Sin` (* (* (`KismetSystemLibrary.GetGameTimeInSeconds`) 2.0) (`self.Floating Speed`))) (`self.Floating Range`))) false false :!label _label))))

(event `self.ReceiveTick`
  (params (DeltaSeconds :type "Float (single-precision)"))
  (bind _returnvalue (* (`KismetMathLibrary.Sin` (* (`KismetSystemLibrary.GetGameTimeInSeconds`) 2.0)) 0.1))
  (`|ExecutionSequence`
    (:`then_0`
      (if (`self.bTimerOn`)
        _))
    (:`then_1`
      (`SceneComponent.K2_AddRelativeRotation` (`self.Cross`) (`KismetMathLibrary.MakeRotator` _returnvalue _returnvalue 1.0) false false)
      (goto _label))))

(event `self.ActivateCollision.OnComponentBeginOverlap`
  (params (OverlappedComponent :type "PrimitiveComponent Object Reference") (OtherActor :type "Actor Object Reference") (OtherComp :type "PrimitiveComponent Object Reference") (OtherBodyIndex :type Integer) (bFromSweep :type Boolean) (SweepResult :type "HitResult Structure (by ref)"))
  (if (`self.ActorHasTag` OtherActor "Player")
    (`KismetSystemLibrary.PrintString` (`KismetStringLibrary.Concat_StrStr` (`KismetSystemLibrary.GetDisplayName` OtherActor) "is" "Overlap"))
    (if (not (`self.bTimerOn`))
      (`self.Timer`))))

(event `Timer`
  (`self.Heal`)
  (set `self.bTimerOn` true)
  (`KismetSystemLibrary.Delay` (`self.HealPackCoolTime`))
  (`ActorComponent.Deactivate` (`self.HealEffect`))
  (`SceneComponent.SetVisibility` (`self.Cross`) true false)
  (set `self.bTimerOn` false))

(event `Heal`
  (bind _returnvalue (`self.K2_GetActorLocation`))
  (bind _healactors (`self.HealActors`))
  (bind _healactors_2 (`self.HealActors`))
  (`KismetArrayLibrary.Array_Clear` (`self.HealActors`))
  (`GameplayStatics.PlaySoundAtLocation` null (`self.K2_GetActorLocation`) (struct) 1.0 1.0 0.2 null null null null)
  (`ActorComponent.Activate` (`self.HealEffect`) false)
  (`SceneComponent.SetVisibility` (`self.Cross`) false false)
  (bind _outhits (`KismetSystemLibrary.SphereTraceMultiForObjects` _returnvalue _returnvalue (`self.Radius`) (`|MakeArray` "ObjectTypeQuery3" :!type "EObjectTypeQuery Enum")))
  (for _array_element _outhits
    (bind (_bblockinghit _binitialoverlap _time _distance _location _impactpoint _normal _impactnormal _physmat _hitactor) (`GameplayStatics.BreakHitResult` _array_element))
    (if (`self.ActorHasTag` _hitactor "Player")
      (if (not (`KismetArrayLibrary.Array_Contains` _healactors _hitactor))
        (`KismetArrayLibrary.Array_Add` _healactors _hitactor))))
  (for _index (range (+ (`KismetArrayLibrary.Array_LastIndex` _healactors_2) 1))
    (`KismetSystemLibrary.PrintString` (`KismetSystemLibrary.GetDisplayName` (`|GetArrayItem` _healactors_2 _index)))))

(fn `RotationCross`)

(fn `UserConstructionScript`)